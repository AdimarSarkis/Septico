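; Interactable wooden door Blueprint that toggles between open and closed through the INTERAGIR event, with a one-second cooldown.
; Opening and closing each play a sound at the door and run a Timeline forward or in reverse, smoothly driving the pivot's yaw up to 100 degrees.
; BeginPlay caches the player character and, for doors starting open, sets the pivot's relative Z location to 100 rather than rotating it.
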(event `self.ReceiveBeginPlay`
  (bind _asbp_third_person_character (cast `/Game/ThirdPerson/Blueprints/BP_ThirdPersonCharacter` (`GameplayStatics.GetPlayerCharacter` 0)))
  (set `self.Player` _asbp_third_person_character)
  (if (not (`self.Porta_Fechada`))
    (`SceneComponent.K2_SetRelativeLocation` (`self.ROTAÇÃO`) (0.0 0.0 100.0) false false)))

(event `AbrirPorta`
  (set `self.Porta_Fechada` false)
  (`GameplayStatics.PlaySoundAtLocation` "/Game/BLUEPRINTS/BP_INTERAGIR/Porta-Madeira/Som-AbrirPorta/Porta_Abrindo_06_Cue.Porta_Abrindo_06_Cue" (`SceneComponent.K2_GetComponentLocation` (`self.Porta-de-Madeira`)) (struct) 1.0 1.0 0.0 null null null null)
  (bind (_direction _suavizar_porta) (`Timeline|Timeline` :!label _label)
    (:`Update`
      (`SceneComponent.K2_SetRelativeRotation` (`self.ROTAÇÃO`) (`KismetMathLibrary.MakeRotator` 0.0 0.0 (* _suavizar_porta 100.0)) false false))))

(event `FecharPorta`
  (set `self.Porta_Fechada` true)
  (`GameplayStatics.PlaySoundAtLocation` "/Game/BLUEPRINTS/BP_INTERAGIR/Porta-Madeira/Som-FecharPorta/Porta_Fechando_06_Cue.Porta_Fechando_06_Cue" (`SceneComponent.K2_GetComponentLocation` (`self.Porta-de-Madeira`)) (struct) 1.0 1.0 0.0 null null null null)
  (goto _label :!via `Reverse`))

(event `/Game/BLUEPRINTS/BP_INTERAGIR/BPI_INTERAGIR.INTERAGIR`
  (if (`self.Posso Interagir?`)
    (set `self.Posso Interagir?` false)
    (if (`self.Porta_Fechada`)
      (`self.AbrirPorta`)
      (else
        (`self.FecharPorta`)))
    (`KismetSystemLibrary.Delay` 1.0)
    (set `self.Posso Interagir?` true)))

(fn `UserConstructionScript`)