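; BPC_INTERAGIR is an interaction component that lets the player interact with the actor the camera is looking at.
; On BeginPlay it casts the player pawn to BP_ThirdPersonCharacter and caches it.
; The INTERACAO event line-traces from the follow camera along its forward vector, up to a configurable interaction distance.
; On a hit, it sends the INTERAGIR interface message to that actor, leaving the Actor argument empty.
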(event `self.ReceiveBeginPlay`
  ;[0.2435 0.5573 0.3396 0.5 50] INTERAÇÃO
  (bind _asbp_third_person_character (cast `/Game/ThirdPerson/Blueprints/BP_ThirdPersonCharacter` (`GameplayStatics.GetPlayerPawn` 0)))
  (set `self.Player` _asbp_third_person_character))

(event `INTERACAO`
  (bind _followcamera (`/Game/ThirdPerson/Blueprints/BP_ThirdPersonCharacter.FollowCamera` (`self.Player`)))
  (bind _returnvalue (`SceneComponent.K2_GetComponentLocation` _followcamera))
  ;[0.2435 0.5573 0.3396 0.5 50] INTERAÇÃO
  (bind (_outhit _returnvalue_2) (`KismetSystemLibrary.LineTraceSingle` _returnvalue (+ _returnvalue (* (`KismetMathLibrary.GetForwardVector` (`SceneComponent.K2_GetComponentRotation` _followcamera)) (`self.Distancia de interação`))) "TraceTypeQuery3"))
  (if _returnvalue_2
    (bind _output_get (set `self.Actor` null))
    (message `/Game/BLUEPRINTS/BP_INTERAGIR/BPI_INTERAGIR.INTERAGIR` (`.HitActor` (`GameplayStatics.BreakHitResult` _outhit)) _output_get)))