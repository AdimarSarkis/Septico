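; Master NPC Blueprint for dialogue, with proximity-driven interaction widgets.
; On BeginPlay it passes its LogicaDialogo to its AI_NPC_DIALOGO controller, and INTERAGIR calls InicioDialogo on that controller to start the dialogue.
; Two trigger boxes, BOXE and BOXSETA, show and hide the E interaction prompt and the SETA arrow widget, respectively, on overlap, only when the overlapping actor equals Mesh.
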(event `self.ReceiveBeginPlay`
  (bind _asai_npc_dialogo (cast `/Game/BLUEPRINTS/BP_DIALOGO/BP_NPC/AI_NPC_DIALOGO` (`AIBlueprintHelperLibrary.GetAIController` self)))
  (set `/Game/BLUEPRINTS/BP_DIALOGO/BP_NPC/AI_NPC_DIALOGO.LogicaDialogo` (`self.Logica Dialogo`) _asai_npc_dialogo))

(event `/Game/BLUEPRINTS/BP_INTERAGIR/BPI_INTERAGIR.INTERAGIR`
  (params (Actor :type "Actor Object Reference"))
  (bind _asai_npc_dialogo (cast `/Game/BLUEPRINTS/BP_DIALOGO/BP_NPC/AI_NPC_DIALOGO` (`AIBlueprintHelperLibrary.GetAIController` self)))
  (`/Game/BLUEPRINTS/BP_DIALOGO/BP_NPC/AI_NPC_DIALOGO.InicioDialogo` _asai_npc_dialogo))

(event `self.BOX-E.OnComponentBeginOverlap`
  (params (OverlappedComponent :type "PrimitiveComponent Object Reference") (OtherActor :type "Actor Object Reference") (OtherComp :type "PrimitiveComponent Object Reference") (OtherBodyIndex :type Integer) (bFromSweep :type Boolean) (SweepResult :type "HitResult Structure (by ref)"))
  ;[0 0.15 0.03305 0.5] COLOCANDO O WIDGET DE INTERAÇÃO
  (if (== OtherActor (`self.Mesh`))
    (`SceneComponent.SetVisibility` (`self.E`) true false)))

(event `self.BOX-E.OnComponentEndOverlap`
  (params (OverlappedComponent :type "PrimitiveComponent Object Reference") (OtherActor :type "Actor Object Reference") (OtherComp :type "PrimitiveComponent Object Reference") (OtherBodyIndex :type Integer))
  ;[0 0.15 0.03305 0.5] COLOCANDO O WIDGET DE INTERAÇÃO
  (if (== OtherActor (`self.Mesh`))
    (`SceneComponent.SetVisibility` (`self.E`) false false)))

(event `self.BOX-SETA.OnComponentBeginOverlap`
  (params (OverlappedComponent :type "PrimitiveComponent Object Reference") (OtherActor :type "Actor Object Reference") (OtherComp :type "PrimitiveComponent Object Reference") (OtherBodyIndex :type Integer) (bFromSweep :type Boolean) (SweepResult :type "HitResult Structure (by ref)"))
  ;[0.15 0.000781 0.000781 0.5] COLOCANDO A WIDGET SETA
  (if (== OtherActor (`self.Mesh`))
    (`SceneComponent.SetVisibility` (`self.SETA`) true false)))

(event `self.BOX-SETA.OnComponentEndOverlap`
  (params (OverlappedComponent :type "PrimitiveComponent Object Reference") (OtherActor :type "Actor Object Reference") (OtherComp :type "PrimitiveComponent Object Reference") (OtherBodyIndex :type Integer))
  ;[0.15 0.000781 0.000781 0.5] COLOCANDO A WIDGET SETA
  (if (== OtherActor (`self.Mesh`))
    (`SceneComponent.SetVisibility` (`self.SETA`) false false)))

(fn `UserConstructionScript`)